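; Pickable lantern item that the BP_PlayerGinger character can equip and hold in hand.
; EquipItem sets the item mesh, trigger sphere and handle to ignore all collision, then attaches to the player mesh's ItemHandSocket.
; The attach result sets the player's IsHoldingItem flag.
; UseItem is empty, and a node to turn off mesh physics simulation is left unconnected.
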(event EventBeginPlay
  (|CallParentFunction) ; This node is disabled and will not be called.\nDrag off pins to build functionality.
)

(event Collision|EventActorBeginOverlap
  (params (OtherActor :type Actor%20Object%20Reference))
  (|CallParentFunction OtherActor) ; This node is disabled and will not be called.\nDrag off pins to build functionality.
)

(event EventTick
  (params (DeltaSeconds :type Float%20%28single-precision%29))
  (|CallParentFunction DeltaSeconds) ; This node is disabled and will not be called.\nDrag off pins to build functionality.
)

(event EventUseItem)

(event EventEquipItem
  (Collision|SetCollisionResponsetoAllChannels (Variables|Default|GetItemMesh) "ECR_Ignore")
  (Collision|SetCollisionResponsetoAllChannels (Variables|Default|GetHandle) "ECR_Ignore")
  (bind _asbp_player_ginger (Utilities|Casting|CastToBP_PlayerGinger (Game|GetPlayerCharacter 0)))
  (bind _returnvalue (Transformation|AttachComponentToComponent self (Variables|/Script/Engine.Character|GetMesh _asbp_player_ginger) "ItemHandSocket" "SnapToTarget" "KeepRelative" "KeepRelative" true))
  (Variables|/Game/Blueprints/Characters/Ginger/BP_PlayerGinger.BP_PlayerGinger_C|SetIsHoldingItem _asbp_player_ginger _returnvalue))

(fn ConstructionScript
  (|CallParentFunction))