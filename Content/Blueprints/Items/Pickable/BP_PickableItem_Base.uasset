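; Base pickable item actor that adds itself to the player's inventory when picked up.
; The Pickup event calls FPickup, which casts player character 0 to BP_PlayerGinger and passes ItemName and Amount to its BPCInventory component's AddItem.
; A partial add leaves the remainder as the new Amount, while a full add destroys the actor.
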(event EventBeginPlay)

(event Collision|EventActorBeginOverlap
  (params (OtherActor :type Actor%20Object%20Reference)))

(event EventTick
  (params (DeltaSeconds :type Float%20%28single-precision%29)))

(event EventPickup
  (CallFunction|FPickup))

(fn ConstructionScript)

(fn FPickup
  (bind _asbp_player_ginger (Utilities|Casting|CastToBP_PlayerGinger (Game|GetPlayerCharacter 0)))
  (bind (_bitemadded _remainder) (Default|AddItem (Variables|/Game/Blueprints/Characters/Ginger/BP_PlayerGinger.BP_PlayerGinger_C|GetBPC_Inventory _asbp_player_ginger) (Variables|Default|GetItemName) (Variables|Default|GetAmount)))
  (if _bitemadded
    (if (> _remainder 0)
      (Variables|Default|SetAmount _remainder)
      (else
        (Actor|DestroyActor)))))