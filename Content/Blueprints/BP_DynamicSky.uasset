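; Day/night sky actor that sets sun, moon, atmosphere and sky sphere from a DayTime value.
; All work runs in the Construction Script, with no runtime update.
; It creates a dynamic sky material, then pitches both lights by mapping DayTime against dawn and dusk.
; Day/night checks toggle light visibility and switch atmospheric scattering, applying moon light settings and optional star and moon material parameters at night.
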(event EventBeginPlay)

(event Collision|EventActorBeginOverlap
  (params (OtherActor :type Actor%20Object%20Reference)))

(event EventTick
  (params (DeltaSeconds :type Float%20%28single-precision%29)))

(fn ConstructionScript
  (bind _is_dynmi_skyspherevalid (Basics|InitSkySphereMaterial))
  (if _is_dynmi_skyspherevalid
    (Utilities|FlowControl|Sequence
      (:then_1
        (Basics|HandleSunRotation)
        (Basics|HandleMoonRotation))
      (:then_2
        (Basics|HandleVisibility))
      (:then_3
        (Night|HandleNightSettings)))))

(fn InitSkySphereMaterial
  (bind _returnvalue (Rendering|Material|CreateDynamicMaterialInstance (Variables|Default|GetSM_SkySphere) 0 "/Game/Materials/Sky/MI_DynamicSkySphere.MI_DynamicSkySphere" "None" :!class /Script/Engine.PrimitiveComponent))
  (bind _output_get (Variables|Default|SetCreated_DynMI_SkySphere _returnvalue))
  (return (Utilities|IsValid _output_get)))

(fn HandleSunRotation
  (Transformation|SetWorldRotation (Variables|Default|GetSunLight) (Math|Rotator|MakeRotator 0.0 (Math|Float|MapRangeUnclamped (Variables|Basics|GetDayTime) (Variables|Basics|GetDawnTime) (Variables|Basics|GetDuskTime) 0.0 -1.8e+02) (Variables|Basics|GetSunMoonZRotation)) false false))

(fn HandleMoonRotation
  ;[1 1 1] Moon Rotation after Dusk
  (Transformation|SetWorldRotation (Variables|Default|GetMoonLight) (Math|Rotator|MakeRotator 0.0 (Math|Float|MapRangeUnclamped (Variables|Basics|GetDayTime) (+ (Variables|Basics|GetDuskTime) 0.3) 24.0 -1.8e+02 -9e+01) 0.0) false false)
  ;[1 1 1] Moon Rotation before Dawn
  (Transformation|SetWorldRotation (Variables|Default|GetMoonLight) (Math|Rotator|MakeRotator 0.0 (Math|Float|MapRangeUnclamped (Variables|Basics|GetDayTime) 0.0 (+ (Variables|Basics|GetDawnTime) 0.3) -9e+01 0.0) (Variables|Basics|GetSunMoonZRotation)) false false))

(fn HandleVisibility
  (Rendering|SetVisibility (Variables|Default|GetSunLight) (Utilities|IsDayTime) false)
  (Rendering|SetVisibility (Variables|Default|GetMoonLight) (Utilities|IsNightTime) false))

(fn HandleNightSettings
  (bind _skyatmosphere (Variables|Default|GetSkyAtmosphere))
  (bind _skyatmosphere_2 (Variables|Default|GetSkyAtmosphere))
  (bind _moonlight (Variables|Default|GetMoonLight))
  (if (Utilities|IsNightTime)
    (Utilities|FlowControl|Sequence
      (:then_0
        (Rendering|Components|Light|SetIntensity _moonlight (Variables|Night|GetMoonLightIntensity))
        (Rendering|Components|Light|SetLightColor _moonlight (Variables|Night|GetMoonLightColor) true)
        (Class|DirectionalLightComponent|SetLightSourceAngle _moonlight (Variables|Night|GetMoonLightSourceAngle))
        (Class|LightComponent|SetTemperature _moonlight (Variables|Night|GetMoonLightTemperature)))
      (:then_1
        (Class|SkyAtmosphereComponent|SetRayleighScattering _skyatmosphere_2 (Variables|Night|GetNightTimeRayScattering))
        (Class|SkyAtmosphereComponent|SetMultiScatteringFactor _skyatmosphere_2 (Variables|Night|GetNightTimeMultiScattering)))
      (:then_2
        ;[1 1 1] Turn Stars on/off
        (Rendering|Material|SetScalarParameterValue (Variables|Default|GetCreated_DynMI_SkySphere) "IsStarVisible" (Math|Float|SelectFloat 1.0 0.0 (Variables|Night|GetShouldShowStars)) :!class /Script/Engine.MaterialInstanceDynamic))
      (:then_3
        ;[1 1 1] Turn Moon on/off
        (Rendering|Material|SetScalarParameterValue (Variables|Default|GetCreated_DynMI_SkySphere) "IsMoonVisible" (Math|Float|SelectFloat 1.0 0.0 (Variables|Night|GetShouldShowMoon)) :!class /Script/Engine.MaterialInstanceDynamic)
        (Rendering|Material|SetVectorParameterValue (Variables|Default|GetCreated_DynMI_SkySphere) "MoonBasicSettings" (Utilities|Struct|MakeLinearColor (/ (Variables|Night|GetMoonScale) 1e+01) (Variables|Night|GetMoonStaticRotation) (Variables|Night|GetMoonBrightness) 1.0) :!class /Script/Engine.MaterialInstanceDynamic)
        (Rendering|Material|SetVectorParameterValue (Variables|Default|GetCreated_DynMI_SkySphere) "MoonTint" (Variables|Night|GetMoonTint) :!class /Script/Engine.MaterialInstanceDynamic)))
    (else
      (Class|SkyAtmosphereComponent|SetRayleighScattering _skyatmosphere "(R=0.174647,G=0.407240,B=1.000000,A=1.000000)")
      (Class|SkyAtmosphereComponent|SetMultiScatteringFactor _skyatmosphere 1.0)
      ;[1 1 1] Hide moon and stars on daytime
      (Rendering|Material|SetScalarParameterValue (Variables|Default|GetCreated_DynMI_SkySphere) "IsStarVisible" 0.0 :!class /Script/Engine.MaterialInstanceDynamic)
      (Rendering|Material|SetScalarParameterValue (Variables|Default|GetCreated_DynMI_SkySphere) "IsMoonVisible" 0.0 :!class /Script/Engine.MaterialInstanceDynamic))))