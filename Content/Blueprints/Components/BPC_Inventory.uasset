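; Inventory component that stores items in a slot array sized from CkrunPlayerController and handles adding, using, equipping and removing them.
; AddItem sets a matching partial stack to max or takes an empty slot, recursing on overflow and returning any remainder.
; UseItem and EquipItem call the first world actor of the item's class, spawning one if none exists; only use decrements quantity.
; Slot changes refresh the matching W_InventoryMenu grid slot.
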(event EventBeginPlay
  (bind _asckrun_player_controller (Utilities|Casting|CastToCkrunPlayerController (Game|GetPlayerController 0)))
  (Utilities|Array|Resize (Variables|Default|GetInventorySlots) (Class|CkrunPlayerController|GetInventorySlots _asckrun_player_controller))
  (bind _asw_inventory_menu (Utilities|Casting|CastToW_InventoryMenu (Class|CkrunPlayerController|GetInventoryWidget _asckrun_player_controller)))
  (Variables|Default|SetWInventoryMenu _asw_inventory_menu))

(fn AddItem
  (params (ItemData :type S%20Item%20Data%20Structure) (Quantity :type Integer))
  (bind (_itemname _icon _maxstackqty _canbeused _canbeequipped _class) (Utilities|Struct|BreakS_ItemData ItemData))
  (bind (_bsuccess _index) (CallFunction|CheckforEmptySlot))
  (bind (_bsuccess_2 _index_2) (CallFunction|CheckforEmptySlot))
  (LocalVariables|SetLocalItemData ItemData)
  (LocalVariables|SetLocalItemName _itemname)
  (LocalVariables|SetLocalQuantity Quantity)
  (LocalVariables|SetLocalItemClass _class)
  (bind _output_get (LocalVariables|SetLocalMaxStackQty _maxstackqty))
  (if (> _output_get 0)
    (bind (_bexists _index_3) (CallFunction|CheckforExistingItem (LocalVariables|GetLocalItemName) (LocalVariables|GetLocalMaxStackQty)))
    (if _bexists
      (bind _output_get_2 (LocalVariables|SetLocalIndex _index_3))
      (if (> (+ (.Amount (CallFunction|GetItemDataatIndex _output_get_2)) (LocalVariables|GetLocalQuantity)) (LocalVariables|GetLocalMaxStackQty))
        (LocalVariables|SetLocalQuantity (- (+ (.Amount (CallFunction|GetItemDataatIndex _output_get_2)) (LocalVariables|GetLocalQuantity)) (LocalVariables|GetLocalMaxStackQty)))
        (Utilities|Array|SetArrayElem (Variables|Default|GetInventorySlots) (LocalVariables|GetLocalIndex) (Utilities|Struct|MakeS_InventoryItems (LocalVariables|GetLocalItemName) (LocalVariables|GetLocalMaxStackQty) (LocalVariables|GetLocalItemClass)))
        (CallFunction|UpdateInventorySlot (LocalVariables|GetLocalIndex))
        (bind _remainder (CallFunction|AddItem (LocalVariables|GetLocalItemData) (LocalVariables|GetLocalQuantity)))
        (return true _remainder)
        (else
          (Utilities|Array|SetArrayElem (Variables|Default|GetInventorySlots) (LocalVariables|GetLocalIndex) (Utilities|Struct|MakeS_InventoryItems (LocalVariables|GetLocalItemName) (LocalVariables|GetLocalMaxStackQty) (LocalVariables|GetLocalItemClass)))
          (CallFunction|UpdateInventorySlot (LocalVariables|GetLocalIndex))
          (return true 0)))
      (elif _bsuccess
        (LocalVariables|SetLocalIndex _index)
        (if (> (LocalVariables|GetLocalQuantity) (LocalVariables|GetLocalMaxStackQty))
          (Utilities|Array|SetArrayElem (Variables|Default|GetInventorySlots) (LocalVariables|GetLocalIndex) (Utilities|Struct|MakeS_InventoryItems (LocalVariables|GetLocalItemName) (LocalVariables|GetLocalMaxStackQty) (LocalVariables|GetLocalItemClass)))
          (CallFunction|UpdateInventorySlot (LocalVariables|GetLocalIndex))
          (bind _remainder_2 (CallFunction|AddItem (LocalVariables|GetLocalItemData) (- (LocalVariables|GetLocalQuantity) (LocalVariables|GetLocalMaxStackQty))))
          (return true _remainder_2)
          (else
            (Utilities|Array|SetArrayElem (Variables|Default|GetInventorySlots) (LocalVariables|GetLocalIndex) (Utilities|Struct|MakeS_InventoryItems (LocalVariables|GetLocalItemName) (LocalVariables|GetLocalQuantity) (LocalVariables|GetLocalItemClass)))
            (CallFunction|UpdateInventorySlot (LocalVariables|GetLocalIndex))
            (return true 0)))
        (else
          (return false (LocalVariables|GetLocalQuantity)))))
    (elif _bsuccess_2
      (bind _output_get_3 (LocalVariables|SetLocalIndex _index_2))
      (Utilities|Array|SetArrayElem (Variables|Default|GetInventorySlots) _output_get_3 (Utilities|Struct|MakeS_InventoryItems (LocalVariables|GetLocalItemName) 1 (LocalVariables|GetLocalItemClass)))
      (CallFunction|UpdateInventorySlot (LocalVariables|GetLocalIndex))
      (if (> (- (LocalVariables|GetLocalQuantity) 1) 0)
        (bind _remainder_3 (CallFunction|AddItem (LocalVariables|GetLocalItemData) (- (LocalVariables|GetLocalQuantity) 1)))
        (return true _remainder_3)
        (else
          (return true 0)))
      (else
        ;[1 1 1 0] No free slots
        (return false (LocalVariables|GetLocalQuantity))))))

(fn CheckforEmptySlot
  (bind (_array_element _array_index) (Utilities|Array|ForEachLoopwithBreak (Variables|Default|GetInventorySlots) :!label _label)
    (:LoopBody
      (if (== (.ItemName (Utilities|Struct|BreakS_InventoryItems _array_element)) "")
        (LocalVariables|SetLocalSlotFound true)
        (LocalVariables|SetLocalIndex _array_index)
        (goto _label Break)
        (else
          (LocalVariables|SetLocalSlotFound false))))
    (:Completed
      (return (LocalVariables|GetLocalSlotFound) (LocalVariables|GetLocalIndex)))))

(fn GetItemDataatIndex
  (params (Index :type Integer))
  (bind _inventoryslots (Variables|Default|GetInventorySlots))
  (bind _output (Utilities|Array|Get(acopy) _inventoryslots Index))
  (bind (_itemname _quantity _itemclass) (Utilities|Struct|BreakS_InventoryItems _output))
  (return _itemname _quantity _itemclass))

(fn UpdateInventorySlot
  (params (Index :type Integer))
  (bind _asckrun_player_controller (Utilities|Casting|CastToCkrunPlayerController (Game|GetPlayerController 0)))
  (bind _asw_inventory_menu (Utilities|Casting|CastToW_InventoryMenu (Class|CkrunPlayerController|GetInventoryWidget _asckrun_player_controller)))
  (Default|UpdateSlot (Utilities|Array|Get(acopy) (Variables|/Game/UMG/Inventory/W_InventoryGrid.W_InventoryGrid_C|GetSlotsArray (Variables|/Game/UMG/Inventory/W_InventoryMenu.W_InventoryMenu_C|GetW_InventoryGrid _asw_inventory_menu)) Index)))

(fn CheckforExistingItem
  (params (ItemName :type Name) (MaxStackAmount :type Integer))
  (bind (_array_element _array_index) (Utilities|Array|ForEachLoopwithBreak (Variables|Default|GetInventorySlots) :!label _label)
    (:LoopBody
      (if (and (== (.ItemName (Utilities|Struct|BreakS_InventoryItems _array_element)) ItemName) (< (.Quantity (Utilities|Struct|BreakS_InventoryItems _array_element)) MaxStackAmount))
        (LocalVariables|SetLocalbExists true)
        (LocalVariables|SetLocalIndex _array_index)
        (goto _label Break)
        (else
          (LocalVariables|SetLocalbExists false))))
    (:Completed
      (return (LocalVariables|GetLocalbExists) (LocalVariables|GetLocalIndex)))))

(fn UseItem
  (params (Index :type Integer))
  (bind _output_get (LocalVariables|SetLocalIndex Index))
  (if (> (.Amount (CallFunction|GetItemDataatIndex _output_get)) 0)
    (bind _returnvalue (Actor|GetActorOfClass (.ItemClass (CallFunction|GetItemDataatIndex _output_get))))
    (Utilities|IsValid _returnvalue
      (:Is%20Valid
        (Default|UseItem _returnvalue))
      (:Is%20Not%20Valid
        (bind _returnvalue_2 (Game|SpawnActorfromClass (.ItemClass (CallFunction|GetItemDataatIndex _output_get)) (Math|Transform|MakeTransform "0, 0, 0" "0, 0, 0" "1.000000,1.000000,1.000000") "Undefined" "MultiplyWithRoot" 0 0))
        (Default|UseItem _returnvalue_2)))
    (CallFunction|RemoveItem (LocalVariables|GetLocalIndex))
    (Default|CloseDropDownMenu (Variables|Default|GetWInventoryMenu))))

(fn EquipItem
  (params (Index :type Integer))
  (bind _output_get (LocalVariables|SetLocalIndex Index))
  (bind _returnvalue (Actor|GetActorOfClass (.ItemClass (CallFunction|GetItemDataatIndex _output_get))))
  (Utilities|IsValid _returnvalue
    (:Is%20Valid
      (Default|EquipItem _returnvalue))
    (:Is%20Not%20Valid
      (bind _returnvalue_2 (Game|SpawnActorfromClass (.ItemClass (CallFunction|GetItemDataatIndex _output_get)) (Math|Transform|MakeTransform "0, 0, 0" "0, 0, 0" "1.000000,1.000000,1.000000") "Undefined" "MultiplyWithRoot" (Game|GetPlayerCharacter 0) 0))
      (Default|EquipItem _returnvalue_2))))

(fn RemoveItem
  (params (Index :type Integer))
  (LocalVariables|SetLocalIndex Index)
  (if (> (.Amount (CallFunction|GetItemDataatIndex (LocalVariables|GetLocalIndex))) 1)
    (Utilities|Array|SetArrayElem (Variables|Default|GetInventorySlots) (LocalVariables|GetLocalIndex) (Utilities|Struct|MakeS_InventoryItems (.Item%20Name (CallFunction|GetItemDataatIndex (LocalVariables|GetLocalIndex))) (- (.Amount (CallFunction|GetItemDataatIndex (LocalVariables|GetLocalIndex))) 1) (.ItemClass (CallFunction|GetItemDataatIndex (LocalVariables|GetLocalIndex)))))
    (else
      (Utilities|Array|SetArrayElem (Variables|Default|GetInventorySlots) (LocalVariables|GetLocalIndex) (Utilities|Struct|MakeS_InventoryItems "None" 0 0))))
  (CallFunction|UpdateInventorySlot (LocalVariables|GetLocalIndex)))